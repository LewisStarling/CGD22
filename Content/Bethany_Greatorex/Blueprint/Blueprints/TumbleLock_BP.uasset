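; Three-dial combination lock puzzle actor that activates a linked object when the correct passcode is entered.
; Interacting with a dial mesh rotates it one tenth of a turn, plays a click and advances its wrapping 0–9 counter.
; The solution button joins the digits in 3-2-1 order, compares them to Passcode, then calls ObjectToActivate through PuzzleLogicInterface.
; The construction script switches all dial materials between two glyph sets.
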(event `/Game/Bethany_Greatorex/Blueprint/Blueprints/Interaction_BPInterface.InteractWithInteractable`
  (params (HitComponant :type "PrimitiveComponent Object Reference"))
  (`|ExecutionSequence`
    (:`then_0`
      (if (== HitComponant (`self.StaticMesh`))
        (`self.Tumble1Update`)
        (`SceneComponent.K2_AddLocalRotation` HitComponant (struct :`Pitch` 36.0) false false :!label _label)
        (`GameplayStatics.PlaySound2D` "/Game/Bethany_Greatorex/Audio/click.click" 1.0 1.0 0.0 null null)))
    (:`then_1`
      (if (== HitComponant (`self.StaticMesh1`))
        (`self.Tumble2Update`)
        (goto _label)))
    (:`then_2`
      (if (== HitComponant (`self.StaticMesh2`))
        (`self.Tumble3Update`)
        (goto _label)))
    (:`then_3`
      (if (== HitComponant (`self.SolutionButton`))
        (`self.CombinationCheck`)))))

(fn `CombinationCheck`
  (bind _object_to_activate (`self.Object to Activate`))
  (if (`KismetStringLibrary.EqualEqual_StrStr` (`self.Passcode`) (`KismetStringLibrary.Concat_StrStr` (`KismetStringLibrary.Conv_IntToString` (`self.Tumble3Value`)) (`KismetStringLibrary.Conv_IntToString` (`self.Tumble2Value`)) (`KismetStringLibrary.Conv_IntToString` (`self.Tumble1Value`))))
    (`KismetSystemLibrary.PrintString` "Code Correct")
    (`GameplayStatics.PlaySound2D` "/Game/Bethany_Greatorex/Audio/Win_sound.Win_sound" 1.0 1.0 0.0 null null)
    (if (`KismetSystemLibrary.IsValid` (`self.Object to Activate`))
      (if (`KismetSystemLibrary.DoesImplementInterface` _object_to_activate "/Game/Bethany_Greatorex/Blueprint/Blueprints/PuzzleLogicInterface.PuzzleLogicInterface_C")
        (message `/Game/Bethany_Greatorex/Blueprint/Blueprints/PuzzleLogicInterface.Activate` _object_to_activate)
        (else
          (`KismetSystemLibrary.PrintString` "ERROR: Object To Activate Does Not Include PuzzleLogicInterface" true true (struct :`R` 1.0 :`A` 1.0) 5.0)))
      (else
        (`KismetSystemLibrary.PrintString` "ERROR: Object to Activate not set" true true (struct :`R` 1.0 :`A` 1.0) 5.0)))
    (else
      (`KismetSystemLibrary.PrintString` "Code Incorrect"))))

(fn `Tumble1Update`
  (bind _result (`/Engine/EditorBlueprintResources/StandardMacros.IncrementInt` (`self.Tumble1Value`))
    (:`  `
      (if (> _result 9)
        (set `self.Tumble1Value` 0))
      (return))))

(fn `Tumble2Update`
  (bind _result (`/Engine/EditorBlueprintResources/StandardMacros.IncrementInt` (`self.Tumble2Value`))
    (:`  `
      (if (> _result 9)
        (set `self.Tumble2Value` 0))
      (return))))

(fn `Tumble3Update`
  (bind _result (`/Engine/EditorBlueprintResources/StandardMacros.IncrementInt` (`self.Tumble3Value`))
    (:`  `
      (if (> _result 9)
        (set `self.Tumble3Value` 0))
      (return))))

(fn `UserConstructionScript`
  (bind _returnvalue (select `int` (`self.Glyph?`) :`0` "/Game/Bethany_Greatorex/Tex_Materials/TumbleLock_Tex_Mat.TumbleLock_Tex_Mat" :`1` "/Game/Bethany_Greatorex/Tex_Materials/TumbleLock2_Tex_Mat.TumbleLock2_Tex_Mat" :!type "MaterialInterface Object Reference"))
  (`PrimitiveComponent.SetMaterial` (`self.StaticMesh`) 0 _returnvalue)
  (`PrimitiveComponent.SetMaterial` (`self.StaticMesh1`) 0 _returnvalue)
  (`PrimitiveComponent.SetMaterial` (`self.StaticMesh2`) 0 _returnvalue))