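; Swinging axe trap that damages the first-person character when it overlaps the hit box.
; A self-restarting timeline lerps the Scene component between positive and negative SwingOffset, using a separate curve for fast swings.
; Activate and Deactivate toggle TrapActive, so deactivation takes effect when the current swing finishes.
; BeginPlay applies the starting rotation and optionally calls Swing, which still requires TrapActive.
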(event `Swing`
  (bind _swingoffset (`self.SwingOffset`))
  (bind _scene (`self.Scene`))
  (bind _swingoffset_2 (`self.SwingOffset`))
  ;[1 1 1] Axe Swing Logic
  (if (`self.TrapActive?`)
    (bind (_direction _axeswing _axefastswing) (`Timeline|AxeSwing` :!via `PlayFromStart` :!label _label)
      (:`Update`
        (if (not (`self.Fast Swing`))
          (`SceneComponent.K2_SetRelativeRotation` _scene (`KismetMathLibrary.RLerp` (`KismetMathLibrary.MakeRotator` 0.0 _swingoffset) (`KismetMathLibrary.MakeRotator` 0.0 (* _swingoffset -1.0)) _axeswing true) false false)
          (else
            (`SceneComponent.K2_SetRelativeRotation` _scene (`KismetMathLibrary.RLerp` (`KismetMathLibrary.MakeRotator` 0.0 _swingoffset_2) (`KismetMathLibrary.MakeRotator` 0.0 (* _swingoffset_2 -1.0)) _axefastswing) false false))))
      (:`Finished`
        (`self.Swing`)))
    (else
      (goto _label :!via `Stop`))))

(event `self.Box.OnComponentBeginOverlap`
  (params (OverlappedComponent :type "PrimitiveComponent Object Reference") (OtherActor :type "Actor Object Reference") (OtherComp :type "PrimitiveComponent Object Reference") (OtherBodyIndex :type Integer) (bFromSweep :type Boolean) (SweepResult :type "HitResult Structure (by ref)"))
  ;[1 1 1] Damage
  (bind _asfirst_person_character (cast `/Game/Production/Tech/FirstPersonCharacterBlueprints/FirstPersonCharacter` OtherActor))
  (`/Game/Production/Tech/FirstPersonCharacterBlueprints/FirstPersonCharacter.ModifyHealth` _asfirst_person_character (`self.Damage`) false))

(event `self.ReceiveBeginPlay`
  ;[1 1 1] Beginning Offset
  (`self.K2_SetActorRotation` (`KismetMathLibrary.MakeRotator` 0.0 (`self.SwingOffset`)))
  ;[1 1 1] Option to have the axes swinging to begin with and not a trigger
  (if (`self.StartSwinging?`)
    (`self.Swing`)))

(event `/Game/Prototype/Tech/PuzzleBlueprints/BPI_PuzzleLogic.Activate`
  (params (`component ` :type "SceneComponent Object Reference"))
  ;[1 1 1] Triggers
  (set `self.TrapActive?` true)
  (`self.Swing`))

(event `/Game/Prototype/Tech/PuzzleBlueprints/BPI_PuzzleLogic.Deactivate`
  ;[1 1 1] Triggers
  (set `self.TrapActive?` false))

(fn `UserConstructionScript`)