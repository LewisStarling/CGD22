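; Trigger point for the light beam puzzle prototype that switches on or off according to which component is passed to its Activate event.
; A match with its Triggerable component turns that mesh's relay material green, while any other component turns it red.
; Standalone, it sends activate or deactivate messages to ObjectToActivate.
; With UsedInMultipleTrigger set, it only records the state in TriggerActive instead of messaging the target.
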(event `/Game/Prototype/Tech/PuzzleBlueprints/BPI_PuzzleLogic.Activate`
  (params (`component ` :type "SceneComponent Object Reference") (`Light Beam` :type Boolean) (TriggeredBy :type "Actor Object Reference"))
  (bind _object_to_activate_ (`self.Object to activate `))
  (bind _triggerable (`self.Triggerable`))
  (bind _returnvalue (== `component ` (`self.Triggerable`)))
  ;[1 1 1] ACTIVE/DEACTIVE
  (if (`self.used in multiple trigger`)
    (if _returnvalue
      (set `self.trigger active` true)
      (`PrimitiveComponent.SetMaterial` _triggerable 1 "/Game/Prototype/Tech/PuzzleBlueprints/Textures/M_RelayGreen.M_RelayGreen" :!label _label)
      (else
        (set `self.trigger active` false)
        (`PrimitiveComponent.SetMaterial` _triggerable 1 "/Game/Prototype/Tech/PuzzleBlueprints/Textures/M_RelayRed.M_RelayRed" :!label _label_2)))
    (elif _returnvalue
      (message `/Game/Prototype/Tech/PuzzleBlueprints/BPI_PuzzleLogic.Activate` _object_to_activate_ null false null)
      (goto _label)
      (else
        (message `/Game/Prototype/Tech/PuzzleBlueprints/BPI_PuzzleLogic.Deactivate` _object_to_activate_ null)
        (goto _label_2)))))

(fn `UserConstructionScript`)