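; Trigger point for the light beam puzzle prototype that switches a linked object based on which component it receives.
; Its Activate event compares the incoming component to Triggerable and sends ObjectToActivate an activate message on a match, or a deactivate message otherwise.
; When MoreThen1 is set, it instead only records the match in the TriggerToActivte flag, which nothing in this graph reads.
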(event `/Game/Prototype/Tech/PuzzleBlueprints/BPI_PuzzleLogic.Activate`
  (params (`component ` :type "SceneComponent Object Reference") (`Light Beam` :type Boolean) (TriggeredBy :type "Actor Object Reference"))
  (bind _object_to_activate_ (`self.Object to activate `))
  (bind _returnvalue (== `component ` (`self.Triggerable`)))
  ;[1 1 1] ACTIVE/DEACTIVE
  (if (`self.More then 1?`)
    (if _returnvalue
      (set `self.trigger to activte ` true)
      (else
        (set `self.trigger to activte ` false)))
    (elif _returnvalue
      (message `/Game/Prototype/Tech/PuzzleBlueprints/BPI_PuzzleLogic.Activate` _object_to_activate_ null false self)
      (else
        (message `/Game/Prototype/Tech/PuzzleBlueprints/BPI_PuzzleLogic.Deactivate` _object_to_activate_)))))

(fn `UserConstructionScript`)