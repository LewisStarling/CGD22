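; BP_ReflectiveSurface is a light beam puzzle prototype surface that emits a reflected beam when hit.
; Reflect moves the beam effect and audio to the hit point, angling forward and away from the light staff or previous reflector.
; A trace along the beam sends activate, damage and chained Reflect messages to the blocking actor.
; A looping timer clears the Hit flag and switches the beam off unless Reflect promptly sets it again.
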(event `self.ReceiveBeginPlay`
  (bind _lightstart (`self.LightStart`))
  (bind _returnvalue (`GameplayStatics.GetActorOfClass` "/Game/Prototype/Tech/LightBeamPuzzle/BP_LightStaff.BP_LightStaff_C"))
  (set `self.Light Staff` _returnvalue)
  (`FXSystemComponent.SetVectorParameter` _lightstart "LightEnd" (+ (`SceneComponent.K2_GetComponentLocation` _lightstart) (* (`SceneComponent.GetForwardVector` _lightstart) 2000.0)))
  (`FXSystemComponent.SetColorParameter` (`self.LightStart`) "Colour" (struct :`R` 1.0 :`G` 0.963151 :`A` 1.0))
  (`KismetSystemLibrary.K2_SetTimerDelegate` (delegate `LightHit?`) 0.1 true))

(event `LightHit?`
  (set `self.Hit?` false)
  (`KismetSystemLibrary.Delay` 0.01)
  (if (not (`self.Hit?`))
    (`SceneComponent.SetVisibility` (`self.LightStart`) false false)
    (`AudioComponent.Stop` (`self.LightBeam`))))

(event `/Game/Production/Tech/Interfaces/BPI_LightPuzzle.Reflect`
  (params (`Start Location` :type "Vector Structure") (`Double Reflect` :type Boolean) (Reflect :type "Actor Object Reference"))
  (bind _lightstart (`self.LightStart`))
  (bind _lightbeam (`self.LightBeam`))
  (if `Double Reflect`
    (set `self.ActorLocation` Reflect)
    (else
      (set `self.ActorLocation` (`self.Light Staff`))))
  (set `self.Hit?` true)
  (`SceneComponent.K2_SetWorldLocation` _lightbeam `Start Location` false false)
  (if (not (`AudioComponent.IsPlaying` _lightbeam))
    (`AudioComponent.Play` _lightbeam 0.0))
  (`SceneComponent.K2_SetWorldLocation` (`self.LightStart`) `Start Location` false false)
  (`SceneComponent.SetVisibility` (`self.LightStart`) true false)
  (set `self.EndLocation` (+ (`SceneComponent.K2_GetComponentLocation` _lightstart) (* (`SceneComponent.GetForwardVector` _lightstart) 5000.0) (* (`KismetMathLibrary.Conv_RotatorToVector` (`KismetMathLibrary.FindLookAtRotation` `Start Location` (`self.K2_GetActorLocation` (`self.ActorLocation`)))) -1000.0)))
  (`FXSystemComponent.SetVectorParameter` (`self.LightStart`) "LightEnd" (`self.EndLocation`))
  (bind _outhit (`KismetSystemLibrary.LineTraceSingle` (`SceneComponent.K2_GetComponentLocation` (`self.LightStart`)) (`self.EndLocation`) "TraceTypeQuery2"))
  (bind (_bblockinghit _binitialoverlap _time _distance _location _impactpoint _normal _impactnormal _physmat _hitactor _hitcomponent) (`GameplayStatics.BreakHitResult` _outhit))
  (set `self.HitLocation` _location)
  (if _bblockinghit
    (message `/Game/Prototype/Tech/PuzzleBlueprints/BPI_PuzzleLogic.Activate` _hitactor _hitcomponent true self)
    (message `/Game/Production/Tech/Interfaces/BPI_LightPuzzle.Reflect` _hitactor (`self.HitLocation`) true self)
    (`FXSystemComponent.SetVectorParameter` (`self.LightStart`) "LightEnd" (`self.HitLocation`))
    (message `/Game/Production/Tech/Interfaces/BPI_Character.Set Stats` _hitactor 0.25 false)
    (else
      (`FXSystemComponent.SetVectorParameter` (`self.LightStart`) "LightEnd" (`self.EndLocation`)))))

(fn `UserConstructionScript`)