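; BP_LightStaff is a light beam puzzle staff that projects a steerable beam and activates what it hits.
; Each tick, a line trace sets the beam's end point and sends Activate to the hit actor, also changing and printing the character's stats when struck.
; Capsule overlaps toggle interaction on nearby actors.
; Axis inputs yaw the staff, or adjust beam height while nudging it along world X.
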(event `self.ReceiveBeginPlay`
  (bind _returnvalue (`GameplayStatics.GetActorOfClass` "/Game/Production/Tech/FirstPersonCharacterBlueprints/FirstPersonCharacter.FirstPersonCharacter_C"))
  (set `self.Character` _returnvalue)
  (`FXSystemComponent.SetColorParameter` (`self.Light`) "Colour" (struct :`R` 1.0 :`G` 0.78496 :`B` 0.027282 :`A` 1.0))
  (`SceneComponent.SetVisibility` (`self.Light`) true false))

(event `self.ReceiveTick`
  (params (DeltaSeconds :type "Float (single-precision)"))
  (bind _returnvalue (`self.K2_GetActorLocation`))
  (bind _returnvalue_2 (+ _returnvalue (* (+ (`self.GetActorForwardVector`) (`KismetMathLibrary.MakeVector` 0.0 0.0 (`self.MoveValue`))) (`self.Distance `))))
  (set `self.EndDistance` _returnvalue_2)
  (bind _outhit (`KismetSystemLibrary.LineTraceSingle` _returnvalue _returnvalue_2 "TraceTypeQuery2"))
  (set `self.Out Hit Blocking Hit` (`GameplayStatics.BreakHitResult` _outhit))
  (set `self.Out Hit Location` (`.Location` (`GameplayStatics.BreakHitResult` _outhit)))
  (set `self.Out Hit Hit Actor` (`.HitActor` (`GameplayStatics.BreakHitResult` _outhit)))
  (set `self.Out Hit Hit Component` (`.HitComponent` (`GameplayStatics.BreakHitResult` _outhit)))
  (`FXSystemComponent.SetVectorParameter` (`self.Light`) "LightEnd" (select `bool` (`self.Out Hit Blocking Hit`) :`false` (`self.EndDistance`) :`true` (`self.Out Hit Location`)))
  (message `/Game/Prototype/Tech/PuzzleBlueprints/BPI_PuzzleLogic.Activate` (`self.Out Hit Hit Actor`) (`self.Out Hit Hit Component`))
  (if (== (`self.Out Hit Hit Actor`) (`self.Character`))
    (bind _health (message `/Game/Production/Tech/Interfaces/BPI_Character.Set Stats` (`self.Out Hit Hit Actor`) 0.25))
    (bind _output_get (set `self.Health` _health))
    (`KismetSystemLibrary.PrintString` (`KismetStringLibrary.Conv_DoubleToString` _output_get))))

(event `self.Capsule.OnComponentBeginOverlap`
  (params (OverlappedComponent :type "PrimitiveComponent Object Reference") (OtherActor :type "Actor Object Reference") (OtherComp :type "PrimitiveComponent Object Reference") (OtherBodyIndex :type Integer) (bFromSweep :type Boolean) (SweepResult :type "HitResult Structure (by ref)"))
  (message `/Game/Production/Tech/Interfaces/BPI_LightPuzzle.CanInteractWithLight` OtherActor true self))

(event `self.Capsule.OnComponentEndOverlap`
  (params (OverlappedComponent :type "PrimitiveComponent Object Reference") (OtherActor :type "Actor Object Reference") (OtherComp :type "PrimitiveComponent Object Reference") (OtherBodyIndex :type Integer))
  (message `/Game/Production/Tech/Interfaces/BPI_LightPuzzle.CanInteractWithLight` OtherActor false self))

(event `/Game/Production/Tech/Interfaces/BPI_LightPuzzle.Add Movement `
  (params (`Axis Value ` :type "Float (single-precision)"))
  (if (> `Axis Value ` 0.0)
    (set `self.MoveValue` (+ (`self.MoveValue`) (`self.MoveSensitivity`)))
    (`self.K2_AddActorWorldTransform` (`KismetMathLibrary.MakeTransform` (`KismetMathLibrary.MakeVector` `Axis Value `)) :!label _label)
    (elif (not (== `Axis Value ` 0.0))
      (set `self.MoveValue` (- (`self.MoveValue`) (`self.MoveSensitivity`)))
      (goto _label))))

(event `/Game/Production/Tech/Interfaces/BPI_LightPuzzle.Add Rotation`
  (params (`Axis Value` :type "Float (single-precision)"))
  (`self.K2_AddActorWorldRotation` (`KismetMathLibrary.MakeRotator` 0.0 0.0 (* `Axis Value` 0.1))))

(fn `UserConstructionScript`)