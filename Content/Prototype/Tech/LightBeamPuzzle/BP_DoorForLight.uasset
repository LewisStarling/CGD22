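; Door for the light beam puzzle that opens when Activate receives its Triggerable component and can close when it receives another.
; Two timelines move the door vertically by adding their track value as a relative Z offset each update, so movement accumulates.
; Paired DoOnce gates alternate the motions: finishing opening sets HasMoved and re-arms closing, and finishing closing re-arms opening.
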(event `/Game/Prototype/Tech/PuzzleBlueprints/BPI_PuzzleLogic.Activate`
  (params (`component ` :type "SceneComponent Object Reference"))
  (bind _door (`self.Door`))
  (bind _returnvalue (== `component ` (`self.Triggerable`)))
  (set `self.ComponetHit` _returnvalue)
  (if _returnvalue
    (`/Engine/EditorBlueprintResources/StandardMacros.DoOnce` false :!label _label
      (:`Completed`
        (bind (_direction _door_open_z) (`Timeline|Open Door` :!via `PlayFromStart`)
          (:`Update`
            (`SceneComponent.K2_AddRelativeLocation` _door (`KismetMathLibrary.MakeVector` 0.0 0.0 _door_open_z) false false))
          (:`Finished`
            (set `self.Has moved` true)
            (goto _label_2 :!via `Reset`)))))
    (elif (and (`self.Has moved`) (not (`self.ComponetHit`)))
      (`/Engine/EditorBlueprintResources/StandardMacros.DoOnce` false :!label _label_2
        (:`Completed`
          (bind (_direction_2 _door_close_) (`Timeline|DoorClose` :!via `PlayFromStart`)
            (:`Update`
              (`SceneComponent.K2_AddRelativeLocation` _door (`KismetMathLibrary.MakeVector` 0.0 0.0 _door_close_) false false))
            (:`Finished`
              (goto _label :!via `Reset`))))))))

(fn `UserConstructionScript`)