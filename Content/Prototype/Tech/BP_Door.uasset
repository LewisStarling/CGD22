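; Prototype door that lifts open when activated and lowers again when deactivated.
; Activate ignores light-beam triggers and locked doors, otherwise playing the DoorOpen timeline to lerp the Hinge's relative Z up to DoorLiftAmount.
; Deactivate reverses the timeline and sets ResetSound.
; The WheelComplete 2D sound is gated by both ResetSound and a DoOnce with no reset wired, so it plays at most once.
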(event `/Game/Prototype/Tech/PuzzleBlueprints/BPI_PuzzleLogic.Activate`
  (params (`component ` :type "SceneComponent Object Reference") (`Light Beam` :type Boolean) (TriggeredBy :type "Actor Object Reference"))
  (bind _hinge (`self.Hinge`))
  (bind (_relativelocation_x _relativelocation_y) (`KismetMathLibrary.BreakVector` (`SceneComponent.RelativeLocation` _hinge)))
  ;[1 1 1] Door opens
  (if `Light Beam`
    _
    (elif (not (`self.Locked?`))
      (`self.Play Sound`)
      (bind (_direction _dooraxis) (`Timeline|DoorOpen` :!label _label)
        (:`Update`
          (`SceneComponent.K2_SetRelativeLocation` _hinge (`KismetMathLibrary.MakeVector` _relativelocation_x _relativelocation_y (`KismetMathLibrary.Lerp` 0.0 (`self.DoorLiftAmount`) _dooraxis)) false false))))))

(event `/Game/Prototype/Tech/PuzzleBlueprints/BPI_PuzzleLogic.Deactivate`
  (params (`Triggered By` :type "Actor Object Reference"))
  ;[1 1 1] Door opens
  (set `self.Reset Sound ` true)
  (goto _label :!via `Reverse`))

(event `Play Sound`
  (`/Engine/EditorBlueprintResources/StandardMacros.DoOnce` false
    (:`Completed`
      (if (`self.Reset Sound `)
        (`GameplayStatics.PlaySound2D` "/Game/Production/Sounds/TraversablePlatform/WheelComplete.WheelComplete" 1.0 1.0 0.0 null null)
        (set `self.Reset Sound ` false)))))

(fn `UserConstructionScript`)