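; Prototype puzzle statue whose left and right arms each cycle through three poses when the player interacts with them.
; BeginPlay puts both arms in the first rotation, then InteractwithInteractable uses the hit component to pick an arm.
; That arm's state counter selects the rotation, then increments, wraps after three and prints for debugging.
; The first two rotations are shared, the third is side-specific, and no solution check happens here.
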(event `self.ReceiveBeginPlay`
  (`SceneComponent.K2_SetRelativeRotation` (`self.Arm_L`) (`self.Arm Rotation 1`) false false)
  (`SceneComponent.K2_SetRelativeRotation` (`self.Arm_R`) (`self.Arm Rotation 1`) false false))

(event `/Game/Prototype/Tech/PuzzleBlueprints/BPI_Interaction.InteractWithInteractable`
  (params (HitComponant :type "PrimitiveComponent Object Reference"))
  (if (or (== HitComponant (`self.Arm_left`)) (== HitComponant (`self.Arm_Right`)))
    (if (== HitComponant (`self.Arm_left`))
      ;[1 1 1] Setting specific rotations for each arm state
      (switch `int` (`self.Arm State_L`) ; Each arm state
        (:`0`
          (`SceneComponent.K2_SetRelativeRotation` (`self.Arm_L`) (`self.Arm Rotation 1`) false false))
        (:`1`
          (`SceneComponent.K2_SetRelativeRotation` (`self.Arm_L`) (`self.Arm Rotation 2`) false false))
        (:`2`
          (`SceneComponent.K2_SetRelativeRotation` (`self.Arm_L`) (`self.Arm Rotation 3_L`) false false)))
      ;[1 1 1] Checks which state the arm is in
      (bind _output_get (set `self.Arm State_L` (+ (`self.Arm State_L`) 1)))
      (if (not (== _output_get 3))
        (`KismetSystemLibrary.PrintString` (`KismetStringLibrary.Conv_IntToString` (`self.Arm State_L`)))
        (else
          (bind _output_get_2 (set `self.Arm State_L` 0))
          (`KismetSystemLibrary.PrintString` (`KismetStringLibrary.Conv_IntToString` _output_get_2))))
      (else
        ;[1 1 1] Setting specific rotations for each arm state
        (switch `int` (`self.Arm State_R`) ; Each arm state
          (:`0`
            (`SceneComponent.K2_SetRelativeRotation` (`self.Arm_R`) (`self.Arm Rotation 1`) false false))
          (:`1`
            (`SceneComponent.K2_SetRelativeRotation` (`self.Arm_R`) (`self.Arm Rotation 2`) false false))
          (:`2`
            (`SceneComponent.K2_SetRelativeRotation` (`self.Arm_R`) (`self.Arm Rotation 3_R`) false false)))
        ;[1 1 1] Checks which state the arm is in
        (bind _output_get_3 (set `self.Arm State_R` (+ (`self.Arm State_R`) 1)))
        (if (not (== _output_get_3 3))
          (`KismetSystemLibrary.PrintString` (`KismetStringLibrary.Conv_IntToString` (`self.Arm State_R`)))
          (else
            (bind _output_get_4 (set `self.Arm State_R` 0))
            (`KismetSystemLibrary.PrintString` (`KismetStringLibrary.Conv_IntToString` _output_get_4))))))))

(fn `UserConstructionScript`)