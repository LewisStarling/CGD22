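; BP_StatuePuzzle is a prototype statue puzzle actor that rotates pieces when the player interacts, with no solution check.
; It caches the FirstPersonCharacter on BeginPlay.
; On interact, it runs its own short, debug-drawn visibility trace from the player's camera rather than using the passed component.
; Whatever component the trace hits has its name printed and turns 90 degrees locally, without filtering to this actor.
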(event `self.ReceiveBeginPlay`
  (bind _returnvalue (`GameplayStatics.GetActorOfClass` "/Game/Production/Tech/FirstPersonCharacterBlueprints/FirstPersonCharacter.FirstPersonCharacter_C"))
  (set `self.FPCharacter` _returnvalue))

(event `/Game/Prototype/Tech/PuzzleBlueprints/BPI_Interaction.InteractWithInteractable`
  (params (HitComponant :type "PrimitiveComponent Object Reference"))
  (bind _firstpersoncamera (`/Game/Production/Tech/FirstPersonCharacterBlueprints/FirstPersonCharacter.FirstPersonCamera` (`self.FPCharacter`)))
  (bind _returnvalue (`SceneComponent.K2_GetComponentLocation` _firstpersoncamera))
  (set `self.Hit Componant` HitComponant)
  (bind (_outhit _returnvalue_2) (`KismetSystemLibrary.LineTraceSingle` :`Start` _returnvalue :`End` (+ _returnvalue (* (`SceneComponent.GetForwardVector` _firstpersoncamera) 300.0)) :`TraceChannel` "TraceTypeQuery1" :`DrawDebugType` "ForDuration" :`bIgnoreSelf` false))
  (if _returnvalue_2
    (bind _output_get (set `self.Out Hit Hit Component` (`.HitComponent` (`GameplayStatics.BreakHitResult` _outhit))))
    (`KismetSystemLibrary.PrintString` (`KismetSystemLibrary.GetDisplayName` _output_get))
    (`SceneComponent.K2_AddLocalRotation` (`self.Out Hit Hit Component`) (struct :`Yaw` 90.0) false false)))

(fn `UserConstructionScript`)