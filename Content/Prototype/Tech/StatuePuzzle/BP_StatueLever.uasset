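; BP_StatueLever is the lever for a statue puzzle that checks whether the statue arms are set correctly when pulled.
; Each interaction flips the lever's tilt and runs ArmStateCheck, which tallies arms matching their correct state against ArmsWithinWorld.
; A match messages the door and relay through BPI_PuzzleLogic, while a mismatch activates the traps.
; The tally persists in a variable that resets only on failure.
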(event `/Game/Prototype/Tech/PuzzleBlueprints/BPI_Interaction.InteractWithInteractable`
  (params (HitComponant :type "PrimitiveComponent Object Reference"))
  (bind _scene (`self.Scene`))
  (bind _doortoopen (`self.DoorToOpen`))
  ;[1 1 1] Lever visuals
  (`/Engine/EditorBlueprintResources/StandardMacros.FlipFlop`
    (:`A`
      (`SceneComponent.K2_SetRelativeRotation` _scene (struct :`Pitch` 30.0) false false))
    (:`B`
      (`SceneComponent.K2_SetRelativeRotation` _scene (struct :`Pitch` -30.0) false false)))
  ;[1 1 1] Arm state check
  (bind _allarmscorrect_ (`self.ArmStateCheck` (`self.StatueArms`)))
  (if _allarmscorrect_
    ;[1 1 1] Triggers Door Open
    (if (`KismetSystemLibrary.DoesImplementInterface` _doortoopen "/Game/Prototype/Tech/PuzzleBlueprints/BPI_PuzzleLogic.BPI_PuzzleLogic_C")
      (message `/Game/Prototype/Tech/PuzzleBlueprints/BPI_PuzzleLogic.Activate` _doortoopen null false self)
      (message `/Game/Prototype/Tech/PuzzleBlueprints/BPI_PuzzleLogic.Activate` (`self.RelayToActivate`) null false self))
    (else
      ;[1 1 1] Traps trigger
      (message `/Game/Prototype/Tech/PuzzleBlueprints/BPI_PuzzleLogic.Activate` (`self.TrapsToTrigger`) null false self))))

(fn `ArmStateCheck`
  (params (Arm :type "Array of /Game/Prototype/Tech/StatuePuzzle/BP_StatueArmPuzzle Object Reference"))
  (returns (`AllArmsCorrect?` :type Boolean))
  (bind _returnvalue (== (`self.NUMBER OF ARMS CORRECT`) (`self.ArmsWithinWorld`)))
  ;[1 1 1] Yes
  (for _array_element Arm
    (if (== (`/Game/Prototype/Tech/StatuePuzzle/BP_StatueArmPuzzle.ArmState` _array_element) (`/Game/Prototype/Tech/StatuePuzzle/BP_StatueArmPuzzle.CorrectArmState` _array_element))
      (set `self.NUMBER OF ARMS CORRECT` (+ (`self.NUMBER OF ARMS CORRECT`) 1))
      (else
        (set `self.NUMBER OF ARMS CORRECT` (- (`self.NUMBER OF ARMS CORRECT`) 1)))))
  (if _returnvalue
    (return _returnvalue)
    (else
      (set `self.NUMBER OF ARMS CORRECT` 0))))

(fn `UserConstructionScript`)