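; Prototype statue puzzle Blueprint with an arm that cycles through three rotations each time it is interacted with.
; A counter selects the relative rotation for the scene component, then increments and wraps back to zero after the third position.
; Every non-wrapping step sends an activate message to the linked door through BPI_PuzzleLogic, with no check for a correct pose.
; The new state is printed for debugging.
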(event `self.ReceiveBeginPlay`
  (bind _returnvalue (`GameplayStatics.GetActorOfClass` "/Game/Production/Tech/FirstPersonCharacterBlueprints/FirstPersonCharacter.FirstPersonCharacter_C"))
  (set `self.FP_Character` _returnvalue))

(event `/Game/Prototype/Tech/PuzzleBlueprints/BPI_Interaction.InteractWithInteractable`
  (params (HitComponant :type "PrimitiveComponent Object Reference"))
  (bind _doortounlock (`self.DoorToUnlock`))
  (switch `int` (`self.ArmState`)
    (:`0`
      (`SceneComponent.K2_SetRelativeRotation` (`self.Scene`) (`self.ArmRotation1`) false false))
    (:`1`
      (`SceneComponent.K2_SetRelativeRotation` (`self.Scene`) (`self.ArmRotation2`) false false))
    (:`2`
      (`SceneComponent.K2_SetRelativeRotation` (`self.Scene`) (`self.ArmRotation3`) false false)))
  ;[1 1 1] Checks which state the arm is in
  (bind _output_get (set `self.ArmState` (+ (`self.ArmState`) 1)))
  (if (not (== _output_get 3))
    (`KismetSystemLibrary.PrintString` (`KismetStringLibrary.Conv_IntToString` (`self.ArmState`)))
    ;[1 1 1] Opens door
    (if (`KismetSystemLibrary.DoesImplementInterface` _doortounlock "/Game/Prototype/Tech/PuzzleBlueprints/BPI_PuzzleLogic.BPI_PuzzleLogic_C")
      (message `/Game/Prototype/Tech/PuzzleBlueprints/BPI_PuzzleLogic.Activate` _doortounlock))
    (else
      (bind _output_get_2 (set `self.ArmState` 0))
      (`KismetSystemLibrary.PrintString` (`KismetStringLibrary.Conv_IntToString` _output_get_2)))))

(fn `UserConstructionScript`)