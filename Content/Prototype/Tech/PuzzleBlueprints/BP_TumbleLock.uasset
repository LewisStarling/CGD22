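; BP_TumbleLock is a three-tumbler combination lock puzzle with a solution button.
; Interacting with a tumbler mesh rotates it one digit step, plays a click and advances its value, wrapping after nine.
; The button animates via a timeline and compares the digits, ordered tumbler 3-2-1, to Passcode.
; A match activates ObjectToActivate through BPI_PuzzleLogic, while a mismatch activates every trap in TrapsToActivate.
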(event `/Game/Prototype/Tech/PuzzleBlueprints/BPI_Interaction.InteractWithInteractable`
  (params (HitComponant :type "PrimitiveComponent Object Reference"))
  (`|ExecutionSequence`
    (:`then_0`
      (if (== HitComponant (`self.StaticMesh`))
        (`self.Tumble1Update`)
        (`SceneComponent.K2_AddLocalRotation` HitComponant (struct :`Roll` -36.0) false false :!label _label)
        (`GameplayStatics.PlaySound2D` "/Game/Prototype/Tech/Audio/Cue_TumbleClick.Cue_TumbleClick" 1.0 1.0 0.0 null null)))
    (:`then_1`
      (if (== HitComponant (`self.StaticMesh1`))
        (`self.Tumble2Update`)
        (goto _label)))
    (:`then_2`
      (if (== HitComponant (`self.StaticMesh2`))
        (`self.Tumble3Update`)
        (goto _label)))
    (:`then_3`
      (if (== HitComponant (`self.SolutionButton`))
        (`self.CombinationCheck`)
        (`self.SolutionButtonPress`)))))

(event `SolutionButtonPress`
  (bind (_intitiallocation_x _intitiallocation_y _intitiallocation_z) (`KismetMathLibrary.BreakVector` (`self.IntitialLocation`)))
  (if (not (`self.ismoving?`))
    (`GameplayStatics.PlaySoundAtLocation` "/Game/Prototype/Tech/Audio/Cue_ButtonPress.Cue_ButtonPress" (`SceneComponent.K2_GetComponentLocation` (`self.DefaultSceneRoot`)) (struct) 1.0 1.0 0.0 null null null)
    (set `self.ismoving?` true)
    (bind (_direction _spikethrust) (`Timeline|Timeline_0` :!via `PlayFromStart`)
      (:`Update`
        (`SceneComponent.K2_SetRelativeLocation` (`self.SolutionButton`) (`KismetMathLibrary.VLerp` (`self.IntitialLocation`) (`KismetMathLibrary.MakeVector` -27.0 _intitiallocation_y _intitiallocation_z) _spikethrust) false false))
      (:`Finished`
        (set `self.ismoving?` false)))))

(event `self.ReceiveBeginPlay`
  (set `self.IntitialLocation` (`SceneComponent.RelativeLocation` (`self.SolutionButton`))))

(fn `CombinationCheck`
  (bind _object_to_activate (`self.Object to Activate`))
  (if (`KismetStringLibrary.EqualEqual_StrStr` (`self.Passcode`) (`KismetStringLibrary.Concat_StrStr` (`KismetStringLibrary.Conv_IntToString` (`self.Tumble3Value`)) (`KismetStringLibrary.Conv_IntToString` (`self.Tumble2Value`)) (`KismetStringLibrary.Conv_IntToString` (`self.Tumble1Value`))))
    (if (`KismetSystemLibrary.IsValid` (`self.Object to Activate`))
      (if (`KismetSystemLibrary.DoesImplementInterface` _object_to_activate "/Game/Prototype/Tech/PuzzleBlueprints/BPI_PuzzleLogic.BPI_PuzzleLogic_C")
        (message `/Game/Prototype/Tech/PuzzleBlueprints/BPI_PuzzleLogic.Activate` _object_to_activate null false self)))
    (else
      (for _array_element (`self.TrapsToActivate`)
        (if (`KismetSystemLibrary.IsValid` _array_element)
          (if (`KismetSystemLibrary.DoesImplementInterface` _array_element "/Game/Prototype/Tech/PuzzleBlueprints/BPI_PuzzleLogic.BPI_PuzzleLogic_C")
            (message `/Game/Prototype/Tech/PuzzleBlueprints/BPI_PuzzleLogic.Activate` _array_element null false null)))))))

(fn `Tumble1Update`
  (bind _result (`/Engine/EditorBlueprintResources/StandardMacros.IncrementInt` (`self.Tumble1Value`))
    (:`  `
      (if (> _result 9)
        (set `self.Tumble1Value` 0))
      (return))))

(fn `Tumble2Update`
  (bind _result (`/Engine/EditorBlueprintResources/StandardMacros.IncrementInt` (`self.Tumble2Value`))
    (:`  `
      (if (> _result 9)
        (set `self.Tumble2Value` 0))
      (return))))

(fn `Tumble3Update`
  (bind _result (`/Engine/EditorBlueprintResources/StandardMacros.IncrementInt` (`self.Tumble3Value`))
    (:`  `
      (if (> _result 9)
        (set `self.Tumble3Value` 0))
      (return))))

(fn `UserConstructionScript`)