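; PathPlate_BP is a prototype pressure path plate that is either enabled or disabled.
; On BeginPlay it sets Enabled to false if its Box overlaps a PathTool_BP actor, so placed tools determine which plates are off.
; When a FirstPersonCharacter enters the Box, it only prints that state as debug text, with no further gameplay effect.
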(event `self.ReceiveBeginPlay`
  (`/Engine/EditorBlueprintResources/StandardMacros.IsValid` (`|GetArrayItem` (`PrimitiveComponent.GetOverlappingActors` (`self.Box`) "/Game/Prototype/Tech/PressurePath/PathTool_BP.PathTool_BP_C"))
    (:`Is Valid`
      (set `self.Enabled?` false))))

(event `self.ReceiveActorBeginOverlap`
  (params (OtherActor :type "Actor Object Reference")))

(event `self.Box.OnComponentBeginOverlap`
  (params (OverlappedComponent :type "PrimitiveComponent Object Reference") (OtherActor :type "Actor Object Reference") (OtherComp :type "PrimitiveComponent Object Reference") (OtherBodyIndex :type Integer) (bFromSweep :type Boolean) (SweepResult :type "HitResult Structure (by ref)"))
  (cast `/Game/Production/Tech/FirstPersonCharacterBlueprints/FirstPersonCharacter` OtherActor)
  (if (`self.Enabled?`)
    (`KismetSystemLibrary.PrintString` "Enabled")
    (else
      (`KismetSystemLibrary.PrintString` "Disabled"))))

(fn `UserConstructionScript`)