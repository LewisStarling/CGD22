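; PathTool_BP is a prototype spline path tool in the PressurePath tech folder that lines a path with box components.
; The construction script adds one box per spline point, placing them at equal time steps along the spline, ending at its far end.
; On BeginPlay, the actor moves up slightly, then drops back by the same offset after a short delay.
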(event `self.ReceiveBeginPlay`
  (bind (_returnvalue_x _returnvalue_y _returnvalue_z) (`KismetMathLibrary.BreakVector` (`self.K2_GetActorLocation`)))
  (bind (_returnvalue_x_2 _returnvalue_y_2 _returnvalue_z_2) (`KismetMathLibrary.BreakVector` (`self.K2_GetActorLocation`)))
  (`self.K2_SetActorLocation` (`KismetMathLibrary.MakeVector` _returnvalue_x_2 _returnvalue_y_2 (+ _returnvalue_z_2 10.0)))
  (`KismetSystemLibrary.Delay` 0.2)
  (`self.K2_SetActorLocation` (`KismetMathLibrary.MakeVector` _returnvalue_x _returnvalue_y (+ _returnvalue_z -10.0))))

(fn `UserConstructionScript`
  (bind _spline (`self.Spline`))
  (bind _returnvalue (`SplineComponent.GetNumberOfSplinePoints` (`self.Spline`)))
  (for _index (range 1 (+ _returnvalue 1))
    (bind _returnvalue_2 (`AddComponent|NODE_AddBoxComponent-0`))
    (`SceneComponent.K2_SetWorldLocation` _returnvalue_2 (`SplineComponent.GetLocationAtTime` _spline (* (`KismetMathLibrary.Conv_IntToDouble` _index) (/ (`SplineComponent.Duration` _spline) (`KismetMathLibrary.Conv_IntToDouble` _returnvalue))) "World" false) false false)))