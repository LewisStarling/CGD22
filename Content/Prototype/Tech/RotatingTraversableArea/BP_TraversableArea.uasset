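; Rotating platform puzzle actor where four switch events turn nested platforms: innermost alone, inner two, inner three, or all four.
; Looping timers step each rotation through a shared counter while per-ring angle values advance by 90 and wrap.
; Each advance triggers a delayed check for the target combination, which locks the switches on success.
; The BeginRotationAnim timeline, which rotates and moves the whole actor, plays on BeginPlay and after completion.
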(event `RotateInnerMost`
  (if (not (`self.Complete Puzzle`))
    (bind _returnvalue (`KismetSystemLibrary.K2_SetTimerDelegate` (delegate `CE_InnerMostRotation`) 0.01 true))
    (set `self.InnerMostTimer` _returnvalue)
    (`self.Added to Degree Checks ` true)))

(event `Switch2Rots`
  (if (not (`self.Complete Puzzle`))
    (bind _returnvalue (`KismetSystemLibrary.K2_SetTimerDelegate` (delegate `CE_Switch2Rotation`) 0.01 true))
    (set `self.Swtich 2 Timer` _returnvalue)
    (`self.Added to Degree Checks ` true true)))

(event `CE_InnerMostRotation`
  (bind _plug_into_null_references_ (`self.Plug Into Null References `))
  (`self.Rotation` (`self.InnerMostTimer`) (`self.Platform 4(InnerMost)`) _plug_into_null_references_ _plug_into_null_references_ _plug_into_null_references_))

(event `CE_Switch2Rotation`
  (bind _plug_into_null_references_ (`self.Plug Into Null References `))
  (`self.Rotation` (`self.Swtich 2 Timer`) (`self.Platform 4(InnerMost)`) (`self.Platform 3`) _plug_into_null_references_ _plug_into_null_references_))

(event `Switch3Rots`
  (if (not (`self.Complete Puzzle`))
    (bind _returnvalue (`KismetSystemLibrary.K2_SetTimerDelegate` (delegate `CE_Switch3Rotation`) 0.01 true))
    (set `self.Switch 3 Timer` _returnvalue)
    (`self.Added to Degree Checks ` true true true)))

(event `Switch4Rots`
  (if (not (`self.Complete Puzzle`))
    (bind _returnvalue (`KismetSystemLibrary.K2_SetTimerDelegate` (delegate `CE_Switch4Rotation`) 0.01 true))
    (set `self.Switch 4 Timer` _returnvalue)
    (`self.Added to Degree Checks ` true true true true)))

(event `CE_Switch3Rotation`
  (`self.Rotation` (`self.Switch 3 Timer`) (`self.Platform2`) (`self.Platform 3`) (`self.Platform 4(InnerMost)`) (`self.Plug Into Null References `)))

(event `CE_Switch4Rotation`
  (`self.Rotation` (`self.Switch 4 Timer`) (`self.Platform1(OuterMost)`) (`self.Platform2`) (`self.Platform 3`) (`self.Platform 4(InnerMost)`)))

(event `self.ReceiveBeginPlay`
  ;[1 1 1] Rotation After puzzle complete
  (bind (_direction _rotation _location_z _location_x) (`Timeline|Begin Rotation Anim` :`NewTime` (`GameplayStatics.GetWorldDeltaSeconds`) :!label _label)
    (:`Update`
      (`self.K2_AddActorLocalRotation` (`KismetMathLibrary.MakeRotator` 0.0 _rotation))
      (`self.K2_AddActorLocalTransform` (`KismetMathLibrary.MakeTransform` (`KismetMathLibrary.MakeVector` _location_x 0.0 _location_z) (struct) (`SceneComponent.K2_GetComponentScale` (`self.DefaultSceneRoot`)))))))

(event `Check for success`
  (`KismetSystemLibrary.Delay` 0.5)
  (if (and (== (`self.Degree4`) 0) (== (`self.Degree3`) 180) (== (`self.Degree2`) 0) (== (`self.Degree1`) 180))
    (`self.Puzzle Complete`)))

(event `Puzzle Complete`
  ;[1 1 1] Rotation After puzzle complete
  (set `self.Complete Puzzle` true)
  (`KismetSystemLibrary.Delay` 2.0)
  (goto _label))

(fn `Added to Degree Checks `
  (params (`1` :type Boolean) (`2` :type Boolean) (`3` :type Boolean) (`4` :type Boolean))
  (`|ExecutionSequence`
    (:`then_0`
      (if `1`
        (bind _set_degree (`self.Degree Check ` (`self.Degree1`)))
        (set `self.Degree1` _set_degree)
        (`KismetSystemLibrary.PrintString` (`KismetStringLibrary.Concat_StrStr` "1 = " (`KismetStringLibrary.Conv_IntToString` (`self.Degree1`))) true true (struct :`G` 0.66 :`B` 1.0 :`A` 1.0) 20.0)
        (`self.Check for success` :!label _label)))
    (:`then_1`
      (if `2`
        (bind _set_degree_2 (`self.Degree Check ` (`self.Degree2`)))
        (set `self.Degree2` _set_degree_2)
        (`KismetSystemLibrary.PrintString` (`KismetStringLibrary.Concat_StrStr` "2 = " (`KismetStringLibrary.Conv_IntToString` (`self.Degree2`))) true true (struct :`G` 0.66 :`B` 1.0 :`A` 1.0) 20.0)
        (goto _label)))
    (:`then_2`
      (if `3`
        (bind _set_degree_3 (`self.Degree Check ` (`self.Degree3`)))
        (set `self.Degree3` _set_degree_3)
        (`KismetSystemLibrary.PrintString` (`KismetStringLibrary.Concat_StrStr` "3 = " (`KismetStringLibrary.Conv_IntToString` (`self.Degree3`))) true true (struct :`G` 0.66 :`B` 1.0 :`A` 1.0) 20.0)
        (goto _label)))
    (:`then_3`
      (if `4`
        (bind _set_degree_4 (`self.Degree Check ` (`self.Degree4`)))
        (set `self.Degree4` _set_degree_4)
        (`KismetSystemLibrary.PrintString` (`KismetStringLibrary.Concat_StrStr` "4 = " (`KismetStringLibrary.Conv_IntToString` (`self.Degree4`))) true true (struct :`G` 0.66 :`B` 1.0 :`A` 1.0) 20.0)
        (goto _label)))))

(fn `Check rotation `
  (returns (`Does rotation` :type Boolean))
  (if (`self.IsRotating?`)
    (return false)
    (else
      (bind _output_get (set `self.IsRotating?` true))
      (return _output_get))))

(fn `Degree Check `
  (params (`Check Degree` :type Integer))
  (returns (`Set Degree` :type Integer))
  (bind _returnvalue (+ `Check Degree` 90))
  (if (>= _returnvalue (`self.Max Degree`))
    (return 0)
    (else
      (return _returnvalue))))

(fn `Rotation`
  (params (Handle :type "TimerHandle Structure (by ref)") (`staticmesh 1` :type "StaticMeshComponent Object Reference") (`static mesh 2` :type "StaticMeshComponent Object Reference") (`static mesh 3 ` :type "StaticMeshComponent Object Reference") (`static mesh 4 ` :type "StaticMeshComponent Object Reference"))
  (if (not (== (`self.add rotation`) (`self.Max rotation `)))
    (bind _output_get (set `self.add rotation` (+ (`self.add rotation`) 1.0)))
    (if (== _output_get (`self.Max rotation `))
      (`KismetSystemLibrary.K2_ClearAndInvalidateTimerHandle` Handle)
      (set `self.add rotation` 0.0)
      (set `self.IsRotating?` false)
      (else
        (`SceneComponent.K2_AddLocalRotation` `staticmesh 1` (struct :`Yaw` 1.0) false false)
        (`SceneComponent.K2_AddLocalRotation` `static mesh 2` (struct :`Yaw` 1.0) false false)
        (`SceneComponent.K2_AddLocalRotation` `static mesh 3 ` (struct :`Yaw` 1.0) false false)
        (`SceneComponent.K2_AddLocalRotation` `static mesh 4 ` (struct :`Yaw` 1.0) false false)))))

(fn `UserConstructionScript`)