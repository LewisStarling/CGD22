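; Four-button control actor for a rotating traversable-area puzzle.
; On interaction, the hit component selects which rotation BPTraversableArea runs: innermost or one of three switch variants.
; CheckRotation accepts a press only while the area is not rotating, then sets its IsRotating flag.
; After a short delay, a completed puzzle plays the BoxesDrop timeline, which offsets this actor's root vertically.
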(event `self.ReceiveBeginPlay`)

(event `/Game/Prototype/Tech/PuzzleBlueprints/BPI_Interaction.InteractWithInteractable`
  (params (HitComponant :type "PrimitiveComponent Object Reference"))
  (set `self.Hit Componant` HitComponant)
  (`|ExecutionSequence`
    (:`then_0`
      (bind _can_rotate_ (`self.CheckRotation` (`self.Hit Componant`) (`self.button1`)))
      (if _can_rotate_
        (`/Game/Prototype/Tech/RotatingTraversableArea/BP_TraversableArea.RotateInnerMost` (`self.BP_TraversableArea`))
        (`KismetSystemLibrary.Delay` 1.75 :!label _label)
        (if (`/Game/Prototype/Tech/RotatingTraversableArea/BP_TraversableArea.Complete Puzzle` (`self.BP_TraversableArea`))
          (bind (_direction _drop) (`Timeline|boxes drop`)
            (:`Update`
              (`SceneComponent.K2_AddRelativeLocation` (`self.DefaultSceneRoot`) (`KismetMathLibrary.MakeVector` 0.0 0.0 _drop) false false))))))
    (:`then_1`
      (bind _can_rotate__2 (`self.CheckRotation` (`self.Hit Componant`) (`self.button2`)))
      (if _can_rotate__2
        (`/Game/Prototype/Tech/RotatingTraversableArea/BP_TraversableArea.Switch2Rots ` (`self.BP_TraversableArea`))
        (goto _label)))
    (:`then_2`
      (bind _can_rotate__3 (`self.CheckRotation` (`self.Hit Componant`) (`self.button3`)))
      (if _can_rotate__3
        (`/Game/Prototype/Tech/RotatingTraversableArea/BP_TraversableArea.Switch3Rots` (`self.BP_TraversableArea`))
        (goto _label)))
    (:`then_3`
      (bind _can_rotate__4 (`self.CheckRotation` (`self.Hit Componant`) (`self.button4`)))
      (if _can_rotate__4
        (`/Game/Prototype/Tech/RotatingTraversableArea/BP_TraversableArea.Switch4Rots` (`self.BP_TraversableArea`))
        (goto _label)))))

(fn `UserConstructionScript`)