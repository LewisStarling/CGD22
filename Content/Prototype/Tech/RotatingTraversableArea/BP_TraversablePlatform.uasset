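; Rotating ring puzzle of four platforms that becomes a traversable platform when solved.
; Four button events each step one platform's yaw by DefaultRot, wrapped at 180 degrees, store it in a map and animate it by timeline.
; After each turn CheckCorrect compares the map values by index against the Anwser array.
; A match plays the completion sound, locks input, then tilts the root from 90 to 0 pitch while lowering the actor.
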(event `self.ReceiveBeginPlay`
  (bind _platform2 (`self.Platform2`))
  (bind _platform_3 (`self.Platform 3`))
  (bind _platform_4_innermost_ (`self.Platform 4(InnerMost)`))
  (bind _platform1_outermost_ (`self.Platform1(OuterMost)`))
  (bind (_relativerotation_roll _relativerotation_pitch _relativerotation_yaw) (`KismetMathLibrary.BreakRotator` (`SceneComponent.RelativeRotation` _platform1_outermost_)))
  (bind (_relativerotation_roll_2 _relativerotation_pitch_2 _relativerotation_yaw_2) (`KismetMathLibrary.BreakRotator` (`SceneComponent.RelativeRotation` _platform2)))
  (bind (_relativerotation_roll_3 _relativerotation_pitch_3 _relativerotation_yaw_3) (`KismetMathLibrary.BreakRotator` (`SceneComponent.RelativeRotation` _platform_3)))
  (bind (_relativerotation_roll_4 _relativerotation_pitch_4 _relativerotation_yaw_4) (`KismetMathLibrary.BreakRotator` (`SceneComponent.RelativeRotation` _platform_4_innermost_)))
  (`AudioComponent.Stop` (`self.TraversablePlatform`))
  (`AudioComponent.Stop` (`self.WheelComplete`))
  (`BlueprintMapLibrary.Map_Add` (`self.Platform Rotation`) _platform1_outermost_ _relativerotation_yaw)
  (`BlueprintMapLibrary.Map_Add` (`self.Platform Rotation`) _platform2 _relativerotation_yaw_2)
  (`BlueprintMapLibrary.Map_Add` (`self.Platform Rotation`) _platform_3 _relativerotation_yaw_3)
  (`BlueprintMapLibrary.Map_Add` (`self.Platform Rotation`) _platform_4_innermost_ _relativerotation_yaw_4))

(event `Rot Button 1`
  (bind _new_rot_1 (`self.New Rot 1`))
  (if (not (`self.Complete`))
    (bind _output_get (set `self.Rot 1` (mod (`BlueprintMapLibrary.Map_Find` (`self.Platform Rotation`) (`self.Platform1(OuterMost)`)) 180.0)))
    (set `self.New Rot 1` (+ _output_get (`self.Default Rot`)))
    (`BlueprintMapLibrary.Map_Add` (`self.Platform Rotation`) (`self.Platform1(OuterMost)`) _new_rot_1)
    (`KismetSystemLibrary.PrintString` (`KismetStringLibrary.Concat_StrStr` "first " (`KismetStringLibrary.Conv_DoubleToString` _new_rot_1)) true true (struct :`G` 0.66 :`B` 1.0 :`A` 1.0) 4.0)
    (`self.PlayAudio`)
    (bind (_direction _rotation) (`Timeline|Rotate` :!via `PlayFromStart`)
      (:`Update`
        (`SceneComponent.K2_SetRelativeRotation` (`self.Platform1(OuterMost)`) (`KismetMathLibrary.MakeRotator` 0.0 0.0 (`KismetMathLibrary.Lerp` (`self.Rot 1`) (`self.New Rot 1`) _rotation)) false false)
        (set `self.Is Playing` true))
      (:`Finished`
        (set `self.Still` true)
        (`self.Check Correct `)
        (set `self.Is Playing` false)))))

(event `rot button 2`
  (bind _new_rot_2 (`self.New Rot 2`))
  (if (not (`self.Complete`))
    (bind _output_get (set `self.Rot 2` (mod (`BlueprintMapLibrary.Map_Find` (`self.Platform Rotation`) (`self.Platform2`)) 180.0)))
    (set `self.New Rot 2` (+ _output_get (`self.Default Rot`)))
    (`BlueprintMapLibrary.Map_Add` (`self.Platform Rotation`) (`self.Platform2`) _new_rot_2)
    (`KismetSystemLibrary.PrintString` (`KismetStringLibrary.Concat_StrStr` "second " (`KismetStringLibrary.Conv_DoubleToString` _new_rot_2)) true true (struct :`G` 0.66 :`B` 1.0 :`A` 1.0) 4.0)
    (bind (_direction _rotation) (`Timeline|Rotate 2` :!via `PlayFromStart`)
      (:`Update`
        (`SceneComponent.K2_SetRelativeRotation` (`self.Platform2`) (`KismetMathLibrary.MakeRotator` 0.0 0.0 (`KismetMathLibrary.Lerp` (`self.Rot 2`) (`self.New Rot 2`) _rotation)) false false))
      (:`Finished`
        (set `self.Still` true)
        (`self.Check Correct `)))))

(event `Rot Button 3`
  (bind _new_rot_3 (`self.New Rot 3`))
  (if (not (`self.Complete`))
    (bind _output_get (set `self.Rot 3` (mod (`BlueprintMapLibrary.Map_Find` (`self.Platform Rotation`) (`self.Platform 3`)) 180.0)))
    (set `self.New Rot 3` (+ _output_get (`self.Default Rot`)))
    (`BlueprintMapLibrary.Map_Add` (`self.Platform Rotation`) (`self.Platform 3`) _new_rot_3)
    (`KismetSystemLibrary.PrintString` (`KismetStringLibrary.Concat_StrStr` "Third  " (`KismetStringLibrary.Conv_DoubleToString` _new_rot_3)) true true (struct :`G` 0.66 :`B` 1.0 :`A` 1.0) 4.0)
    (bind (_direction _rotation) (`Timeline|Rotate 3` :!via `PlayFromStart`)
      (:`Update`
        (`SceneComponent.K2_SetRelativeRotation` (`self.Platform 3`) (`KismetMathLibrary.MakeRotator` 0.0 0.0 (`KismetMathLibrary.Lerp` (`self.Rot 3`) (`self.New Rot 3`) _rotation)) false false))
      (:`Finished`
        (set `self.Still` true)
        (`self.Check Correct `)))))

(event `Rot Button 4`
  (bind _new_rot_4 (`self.New Rot 4`))
  (if (not (`self.Complete`))
    (bind _output_get (set `self.Rot 4` (mod (`BlueprintMapLibrary.Map_Find` (`self.Platform Rotation`) (`self.Platform 4(InnerMost)`)) 180.0)))
    (set `self.New Rot 4` (+ _output_get (`self.Default Rot`)))
    (`BlueprintMapLibrary.Map_Add` (`self.Platform Rotation`) (`self.Platform 4(InnerMost)`) _new_rot_4)
    (`KismetSystemLibrary.PrintString` (`KismetStringLibrary.Concat_StrStr` "fourth" (`KismetStringLibrary.Conv_DoubleToString` _new_rot_4)) true true (struct :`G` 0.66 :`B` 1.0 :`A` 1.0) 4.0)
    (bind (_direction _rotation) (`Timeline|Rotate 4` :!via `PlayFromStart`)
      (:`Update`
        (`SceneComponent.K2_SetRelativeRotation` (`self.Platform 4(InnerMost)`) (`KismetMathLibrary.MakeRotator` 0.0 0.0 (`KismetMathLibrary.Lerp` (`self.Rot 4`) (`self.New Rot 4`) _rotation)) false false))
      (:`Finished`
        (set `self.Still` true)
        (`self.Check Correct `)))))

(event `Win`
  (bind (_returnvalue_x _returnvalue_y _returnvalue_z) (`KismetMathLibrary.BreakVector` (`self.K2_GetActorLocation`)))
  (bind _defaultsceneroot (`self.DefaultSceneRoot`))
  (bind (_relativerotation_roll _relativerotation_pitch _relativerotation_yaw) (`KismetMathLibrary.BreakRotator` (`SceneComponent.RelativeRotation` _defaultsceneroot)))
  (set `self.Complete` true)
  (set `self.Loc X` _returnvalue_x)
  (set `self.Loc Y ` _returnvalue_y)
  (bind _output_get (set `self.Loc Z` _returnvalue_z))
  (set `self.New Z ` (- _output_get 150.0))
  (`KismetSystemLibrary.Delay` 0.2)
  (bind (_direction _rotate) (`Timeline|RotateToTraverse` :!via `PlayFromStart`)
    (:`Update`
      (`SceneComponent.K2_SetRelativeRotation` _defaultsceneroot (`KismetMathLibrary.MakeRotator` _relativerotation_roll (`KismetMathLibrary.Lerp` 90.0 0.0 _rotate) _relativerotation_yaw) false false)
      (`self.K2_SetActorRelativeLocation` (`KismetMathLibrary.MakeVector` (`self.Loc X`) (`self.Loc Y `) (`KismetMathLibrary.Lerp` (`self.Loc Z`) (`self.New Z `) _rotate))))))

(fn `Check Correct `
  (set `self.Correct` true)
  (for (_array_element _array_index) (`self.Anwser`)
    (bind _values (`BlueprintMapLibrary.Map_Values` (`self.Platform Rotation`)))
    (if (not (== _array_element (`|GetArrayItem` _values _array_index)))
      (set `self.Correct` false)))
  (if (`self.Correct`)
    (`AudioComponent.Play` (`self.WheelComplete`) 0.0)
    (`self.Win`)))

(fn `PlayAudio`
  (if (not (`self.Is Playing`))
    (`AudioComponent.Play` (`self.TraversablePlatform`) 0.0)))

(fn `RotatePlatform`
  (params (Key :type "StaticMeshComponent Object Reference (by ref)"))
  (returns (Out :type "StaticMeshComponent Object Reference"))
  (locals (Platform :type "StaticMeshComponent Object Reference")))

(fn `UserConstructionScript`)