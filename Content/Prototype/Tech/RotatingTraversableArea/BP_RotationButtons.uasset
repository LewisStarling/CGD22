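; BP_RotationButtons is a prototype interactable set of buttons that drives rotation on a linked traversable platform.
; Interaction is accepted only while the platform's Still flag is true, and the flag is cleared before any rotation call.
; The hit component selects a cumulative call chain: Button1 calls RotButton1, Button2 and Button3 add the next functions, and any other component calls all four.
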(event `/Game/Prototype/Tech/PuzzleBlueprints/BPI_Interaction.InteractWithInteractable`
  (params (HitComponant :type "PrimitiveComponent Object Reference"))
  (bind _bp_traversableplatform (`self.BP_TraversablePlatform`))
  (bind _bp_traversableplatform_2 (`self.BP_TraversablePlatform`))
  (bind _bp_traversableplatform_3 (`self.BP_TraversablePlatform`))
  ;[1 1 1] Rotation Interaction
  (if (`/Game/Prototype/Tech/RotatingTraversableArea/BP_TraversablePlatform.Still` (`self.BP_TraversablePlatform`))
    (set `/Game/Prototype/Tech/RotatingTraversableArea/BP_TraversablePlatform.Still` false (`self.BP_TraversablePlatform`))
    (bind _output_get (set `self.Hit` HitComponant))
    (if (== _output_get (`self.button1`))
      (`/Game/Prototype/Tech/RotatingTraversableArea/BP_TraversablePlatform.Rot Button 1` (`self.BP_TraversablePlatform`))
      (elif (== (`self.Hit`) (`self.button2`))
        (`/Game/Prototype/Tech/RotatingTraversableArea/BP_TraversablePlatform.Rot Button 1` _bp_traversableplatform_3)
        (`/Game/Prototype/Tech/RotatingTraversableArea/BP_TraversablePlatform.rot button 2 ` _bp_traversableplatform_3)
        (elif (== (`self.Hit`) (`self.button3`))
          (`/Game/Prototype/Tech/RotatingTraversableArea/BP_TraversablePlatform.Rot Button 1` _bp_traversableplatform)
          (`/Game/Prototype/Tech/RotatingTraversableArea/BP_TraversablePlatform.rot button 2 ` _bp_traversableplatform)
          (`/Game/Prototype/Tech/RotatingTraversableArea/BP_TraversablePlatform.Rot Button 3` _bp_traversableplatform)
          (else
            (`/Game/Prototype/Tech/RotatingTraversableArea/BP_TraversablePlatform.Rot Button 1` _bp_traversableplatform_2)
            (`/Game/Prototype/Tech/RotatingTraversableArea/BP_TraversablePlatform.rot button 2 ` _bp_traversableplatform_2)
            (`/Game/Prototype/Tech/RotatingTraversableArea/BP_TraversablePlatform.Rot Button 3` _bp_traversableplatform_2)
            (`/Game/Prototype/Tech/RotatingTraversableArea/BP_TraversablePlatform.Rot Button 4 ` _bp_traversableplatform_2)))))))

(fn `UserConstructionScript`)