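; Three-wheel rotation puzzle prototype that activates a linked object when every wheel sits at its target position.
; Interacting with one of three buttons starts a looping timer that yaws that layer in steps up to MaxRot, with a shared Rot flag blocking overlapping turns.
; After a delay, the layer's position counter advances and updates TrueWheelStates.
; CheckAll tallies that array, then prints completion and sends ActivateMessage to ObjectToActivate.
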(event `RotFunction`
  (bind _truewheelstates_ (`self.TrueWheelStates `))
  (bind _layer_1_int (`self.Layer 1 Int`))
  (bind _finish (`self.RotFunction()` (`self.Timer`) (`self.Layer1 `)))
  (`KismetSystemLibrary.Delay` 1.5)
  (set `self.Rot` (not _finish))
  (bind _result (`/Engine/EditorBlueprintResources/StandardMacros.IncrementInt` _layer_1_int)
    (:`  `
      (if (== _result 4)
        (set `self.Layer 1 Int` 0)
        (`KismetArrayLibrary.Array_Set` (`self.TrueWheelStates `))
        (elif (== _layer_1_int 1)
          (`KismetArrayLibrary.Array_Set` _truewheelstates_ 0 true)
          (`self.CheckAll()`)
          (else
            (`KismetArrayLibrary.Array_Set` _truewheelstates_)))))))

(event `/Game/Prototype/Tech/PuzzleBlueprints/BPI_Interaction.InteractWithInteractable`
  (params (HitComponant :type "PrimitiveComponent Object Reference"))
  (set `self.Hit Componant` HitComponant)
  (`|ExecutionSequence`
    (:`then_0`
      (bind _returnvalue (`self.Check component` (`self.Button1`))
        (:`component `
          (if _returnvalue
            (bind _returnvalue_2 (`KismetSystemLibrary.K2_SetTimerDelegate` (delegate `RotFunction`) 0.01 true))
            (set `self.Timer` _returnvalue_2)))))
    (:`then_1`
      (bind _returnvalue_3 (`self.Check component` (`self.Button2`))
        (:`component `
          (if _returnvalue_3
            (bind _returnvalue_4 (`KismetSystemLibrary.K2_SetTimerDelegate` (delegate `RotFunction2`) 0.01 true))
            (set `self.Timer2` _returnvalue_4)))))
    (:`then_2`
      (bind _returnvalue_5 (`self.Check component` (`self.Button3`))
        (:`component `
          (if _returnvalue_5
            (bind _returnvalue_6 (`KismetSystemLibrary.K2_SetTimerDelegate` (delegate `RotFunction3`) 0.01 true))
            (set `self.Timer3` _returnvalue_6)))))))

(event `RotFunction2`
  (bind _truewheelstates_ (`self.TrueWheelStates `))
  (bind _layer2int_ (`self.Layer2Int `))
  (bind _finish (`self.RotFunction()` (`self.Timer2`) (`self.Layer2`)))
  (`KismetSystemLibrary.Delay` 1.5)
  (set `self.Rot` (not _finish))
  (bind _result (`/Engine/EditorBlueprintResources/StandardMacros.IncrementInt` _layer2int_)
    (:`  `
      (if (== _result 4)
        (set `self.Layer2Int ` 0)
        (`KismetArrayLibrary.Array_Set` (`self.TrueWheelStates `))
        (elif (== _layer2int_ 3)
          (`KismetArrayLibrary.Array_Set` _truewheelstates_ 1 true)
          (`self.CheckAll()`)
          (else
            (`KismetArrayLibrary.Array_Set` _truewheelstates_ 1)))))))

(event `RotFunction3`
  (bind _layer3int (`self.Layer3Int`))
  (bind _truewheelstates_ (`self.TrueWheelStates `))
  (bind _finish (`self.RotFunction()` (`self.Timer3`) (`self.Layer3`)))
  (`KismetSystemLibrary.Delay` 1.5)
  (set `self.Rot` (not _finish))
  (bind _result (`/Engine/EditorBlueprintResources/StandardMacros.IncrementInt` _layer3int)
    (:`  `
      (if (== _result 4)
        (set `self.Layer3Int` 0)
        (`KismetArrayLibrary.Array_Set` (`self.TrueWheelStates `))
        (elif (== _layer3int 2)
          (`KismetArrayLibrary.Array_Set` _truewheelstates_ 2 true)
          (`self.CheckAll()`)
          (else
            (`KismetArrayLibrary.Array_Set` _truewheelstates_ 2)))))))

(fn `CheckAll()`
  (for _array_element (`self.TrueWheelStates `)
    (if (== _array_element true)
      (`/Engine/EditorBlueprintResources/StandardMacros.IncrementInt` (`self.overallInt`))
      (else
        (`/Engine/EditorBlueprintResources/StandardMacros.DecrementInt` (`self.overallInt`)))))
  (if (== (`self.overallInt`) 3)
    (`KismetSystemLibrary.PrintString` "Puzzle Complete " true true (struct :`R` 1.0 :`G` 0.831943 :`A` 1.0))
    (message `/Game/Prototype/Tech/PuzzleBlueprints/BPI_PuzzleLogic.Activate` (`self.Object to Activate `) null)
    (else
      (set `self.overallInt` 0))))

(fn `RotFunction()`
  (params (Handle :type "TimerHandle Structure (by ref)") (Target :type "SceneComponent Object Reference"))
  (returns (Finish :type Boolean))
  (bind _output_get (set `self.RotationFloat` (+ (`self.RotationFloat`) 1.0)))
  (if (>= _output_get (`self.MaxRot`))
    (`KismetSystemLibrary.K2_ClearAndInvalidateTimerHandle` Handle)
    (set `self.RotationFloat` 0.0)
    (else
      (`SceneComponent.K2_AddLocalRotation` Target (`KismetMathLibrary.MakeRotator` 0.0 0.0 1.0) false false)
      (return true))))

(fn `UserConstructionScript`)