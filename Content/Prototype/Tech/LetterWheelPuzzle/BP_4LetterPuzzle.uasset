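; Four-wheel letter puzzle that activates a linked door when the correct combination is submitted, or triggers linked traps when it is wrong.
; Interacting with a wheel rotates it one step via a timeline and advances its 12-position index, playing a distinct sound when that wheel matches its answer.
; Pressing the button compares all indices, held in maps keyed by wheel mesh, against Answers.
; A Rotating flag blocks input during either animation.
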(event `self.ReceiveBeginPlay`
  (`BlueprintMapLibrary.Map_Add` (`self.Wheel Layers `) (`self.Layer 1`))
  (`BlueprintMapLibrary.Map_Add` (`self.Wheel Layers `) (`self.Layer2`))
  (`BlueprintMapLibrary.Map_Add` (`self.Wheel Layers `) (`self.Layer3`))
  (`BlueprintMapLibrary.Map_Add` (`self.Wheel Layers `) (`self.Layer4`))
  (`self.Add Static Meshes to Map of Answers`))

(event `/Game/Prototype/Tech/PuzzleBlueprints/BPI_Interaction.InteractWithInteractable`
  (params (HitComponant :type "PrimitiveComponent Object Reference"))
  ;[1 1 1] Rotation Functionality
  (if (not (`self.Rotating`))
    (if (== HitComponant (`self.Button`))
      (`GameplayStatics.PlaySound2D` "/Game/Production/Sounds/LetterWheel/LetterWheel.LetterWheel" 1.0 1.0 0.0 null null)
      (bind _all_correct (`self.Check for correct anwser `))
      (if _all_correct
        (`/Game/Prototype/Tech/BP_Door.Activate` (`self.Door To Open `) null false self)
        (else
          (for _array_element (`self.Trap To Trigger`)
            (message `/Game/Prototype/Tech/PuzzleBlueprints/BPI_PuzzleLogic.Activate` _array_element null false self))))
      (set `self.Rotating` true)
      (bind (_direction _location) (`Timeline|ButtonPress` :!via `PlayFromStart`)
        (:`Update`
          (`SceneComponent.K2_SetRelativeLocation` (`self.Button`) (`KismetMathLibrary.MakeVector` 0.0 (`KismetMathLibrary.Lerp` -37.0 -43.0 _location)) false false))
        (:`Finished`
          (set `self.Rotating` false)))
      (else
        (bind (_rotatethis _start _target) (`self.Set Rotation Amount` HitComponant))
        (set `self.Hit Component` _rotatethis)
        (`self.Set Current Number`)
        (`self.Check Correct Turn `)
        (set `self.Rotating` true)
        (bind (_direction_2 _rotate) (`Timeline|RotateWheel` :!via `PlayFromStart`)
          (:`Update`
            (`SceneComponent.K2_SetRelativeRotation` (`self.Hit Component`) (`KismetMathLibrary.MakeRotator` 0.0 (`KismetMathLibrary.Lerp` _start _target _rotate)) false false))
          (:`Finished`
            (set `self.Rotating` false)))))))

(fn `Add Static Meshes to Map of Answers`
  (bind _layernumbers (`self.LayerNumbers`))
  (bind _keys (`BlueprintMapLibrary.Map_Keys` (`self.Wheel Layers `)))
  (for _array_element _keys
    (`BlueprintMapLibrary.Map_Add` _layernumbers _array_element))
  (bind _keys_2 (`BlueprintMapLibrary.Map_Keys` _layernumbers))
  (for _ _keys_2
    _))

(fn `Check Correct Turn `
  (bind _keys (`BlueprintMapLibrary.Map_Keys` (`self.LayerNumbers`)))
  (for (_array_element _array_index) _keys
    (if (== _array_element (`self.Hit Component`))
      (bind _values (`BlueprintMapLibrary.Map_Values` (`self.LayerNumbers`)))
      (if (== (`|GetArrayItem` _values _array_index) (`|GetArrayItem` (`self.Answers`) _array_index))
        (`GameplayStatics.PlaySound2D` "/Game/Production/Sounds/LetterWheel/LetterWheelCorrect.LetterWheelCorrect" 1.0 1.0 0.0 null null)
        (else
          (`GameplayStatics.PlaySound2D` "/Game/Production/Sounds/LetterWheel/LetterWheel.LetterWheel" 1.0 1.0 0.0 null null))))))

(fn `Check for correct anwser `
  (returns (`All Correct` :type Boolean))
  (set `self.Correct` true)
  (for (_array_element _array_index) (`self.Answers`)
    (bind _values (`BlueprintMapLibrary.Map_Values` (`self.LayerNumbers`)))
    (if (not (== _array_element (`|GetArrayItem` _values _array_index)))
      (set `self.Correct` false)))
  (return (`self.Correct`)))

(fn `Set Current Number`
  (bind _layernumbers (`self.LayerNumbers`))
  (bind _keys (`BlueprintMapLibrary.Map_Keys` (`self.LayerNumbers`)))
  (for _array_element _keys
    (if (== _array_element (`self.Hit Component`))
      (`BlueprintMapLibrary.Map_Add` _layernumbers _array_element (+ (`BlueprintMapLibrary.Map_Find` _layernumbers _array_element) 1))
      (if (== (`BlueprintMapLibrary.Map_Find` (`self.LayerNumbers`) _array_element) 12)
        (`BlueprintMapLibrary.Map_Add` (`self.LayerNumbers`) _array_element)))))

(fn `Set Rotation Amount`
  (params (Layer :type "PrimitiveComponent Object Reference"))
  (returns (RotateThis :type "StaticMeshComponent Object Reference") (Start :type "Float (double-precision)") (Target :type "Float (double-precision)"))
  (locals (StartRotation :type "Float (double-precision)") (EndRotation :type "Float (double-precision)"))
  (bind _wheel_layers_ (`self.Wheel Layers `))
  (bind _keys (`BlueprintMapLibrary.Map_Keys` (`self.Wheel Layers `)))
  (for _array_element _keys
    (if (== _array_element Layer)
      (bind _output_get (set `local.StartRotation` (mod (`BlueprintMapLibrary.Map_Find` _wheel_layers_ _array_element) 360.0)))
      (bind _output_get_2 (set `local.EndRotation` (+ _output_get (`self.ROT`))))
      (`BlueprintMapLibrary.Map_Add` _wheel_layers_ _array_element _output_get_2)
      (return _array_element (`local.StartRotation`) (`local.EndRotation`)))))

(fn `UserConstructionScript`)