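; BP_LetterPuzzle is a prototype letter wheel puzzle with five layers that rotate when interacted with.
; Interaction plays a timeline that lerps the hit component's pitch from its current value toward a shared target, ignoring new rotations until finished.
; The target then advances 30 degrees and prints.
; A per-layer map sets a rotation amount on each interaction, but the rotation never uses it.
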(event `self.ReceiveBeginPlay`
  (`BlueprintMapLibrary.Map_Add` (`self.Wheel Layers `) (`self.Layer0`) 0.95)
  (`BlueprintMapLibrary.Map_Add` (`self.Wheel Layers `) (`self.Layer 1`) 1.9)
  (`BlueprintMapLibrary.Map_Add` (`self.Wheel Layers `) (`self.Layer2`) 2.85)
  (`BlueprintMapLibrary.Map_Add` (`self.Wheel Layers `) (`self.Layer3`) 3.8)
  (`BlueprintMapLibrary.Map_Add` (`self.Wheel Layers `) (`self.Layer4`) 4.75))

(event `/Game/Prototype/Tech/PuzzleBlueprints/BPI_Interaction.InteractWithInteractable`
  (params (HitComponant :type "PrimitiveComponent Object Reference"))
  (bind (_relativerotation_roll _relativerotation_pitch) (`KismetMathLibrary.BreakRotator` (`SceneComponent.RelativeRotation` (`self.Hit Component`))))
  (`self.Set Rotation Amount` HitComponant)
  (if (not (`self.Rotating`))
    (set `self.Hit Component` HitComponant)
    (set `self.Rotating` true)
    (bind (_direction _rotate) (`Timeline|RotateWheel` :!via `PlayFromStart`)
      (:`Update`
        (`SceneComponent.K2_SetRelativeRotation` (`self.Hit Component`) (`KismetMathLibrary.MakeRotator` 0.0 (`KismetMathLibrary.Lerp` _relativerotation_pitch (`self.ROT`) _rotate)) false false))
      (:`Finished`
        (set `self.Rotating` false)
        (bind _output_get (set `self.ROT` (+ (`self.ROT`) 30.0)))
        (`KismetSystemLibrary.PrintString` (`KismetStringLibrary.Conv_DoubleToString` _output_get))))))

(fn `Set Rotation Amount`
  (params (Layer :type "PrimitiveComponent Object Reference"))
  (bind _keys (`BlueprintMapLibrary.Map_Keys` (`self.Wheel Layers `)))
  (for _array_element _keys
    (if (== _array_element Layer)
      (set `self.Rotation Amount ` (`BlueprintMapLibrary.Map_Find` (`self.Wheel Layers `) _array_element)))))

(fn `UserConstructionScript`)