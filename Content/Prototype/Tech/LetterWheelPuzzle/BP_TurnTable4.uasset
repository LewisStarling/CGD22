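; Four-layer turntable puzzle, part of a letter wheel prototype, that activates a linked object when every layer sits at its hard-coded target step.
; Interacting with a layer's button starts a looping timer that yaws that layer in one-degree ticks up to MaxRot, with a shared Rot flag gating input.
; After a delay, each turn advances a wrapping step counter and updates TrueWheelStates, which CheckAll tallies whenever a layer reaches its target.
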(event `Rotfun`
  (bind _truewheelstates_ (`self.TrueWheelStates `))
  (bind _layer_1_ (`self.Layer 1 `))
  (bind _finish (`self.RotFunction()` (`self.Timer 0`) (`self.Layer 1`)))
  (`KismetSystemLibrary.Delay` 0.75)
  (set `self.Rot` (not _finish))
  (bind _result (`/Engine/EditorBlueprintResources/StandardMacros.IncrementInt` _layer_1_)
    (:`  `
      (if (== _result (`self.NumberofRots`))
        (set `self.Layer 1 ` 0)
        (`KismetArrayLibrary.Array_Set` (`self.TrueWheelStates `))
        (elif (== _layer_1_ 1)
          (`KismetArrayLibrary.Array_Set` _truewheelstates_ 0 true)
          (`self.CheckAll()`)
          (else
            (`KismetArrayLibrary.Array_Set` _truewheelstates_)))))))

(event `RotFunction`
  (bind _truewheelstates_ (`self.TrueWheelStates `))
  (bind _layer_2__ (`self.Layer 2  `))
  (bind _finish (`self.RotFunction()` (`self.Timer 1`) (`self.Layer2`)))
  (`KismetSystemLibrary.Delay` 0.75)
  (set `self.Rot` (not _finish))
  (bind _result (`/Engine/EditorBlueprintResources/StandardMacros.IncrementInt` _layer_2__)
    (:`  `
      (if (== _result (`self.NumberofRots`))
        (set `self.Layer 2  ` 0)
        (`KismetArrayLibrary.Array_Set` (`self.TrueWheelStates `) 1)
        (elif (== _layer_2__ 3)
          (`KismetArrayLibrary.Array_Set` _truewheelstates_ 1 true)
          (`self.CheckAll()`)
          (else
            (`KismetArrayLibrary.Array_Set` _truewheelstates_ 1)))))))

(event `/Game/Prototype/Tech/PuzzleBlueprints/BPI_Interaction.InteractWithInteractable`
  (params (HitComponant :type "PrimitiveComponent Object Reference"))
  (set `self.Hit Componant` HitComponant)
  (`|ExecutionSequence`
    (:`then_0`
      (bind _returnvalue (`self.Check component` (`self.Button1`))
        (:`component `
          (if _returnvalue
            (bind _returnvalue_2 (`KismetSystemLibrary.K2_SetTimerDelegate` (delegate `Rotfun`) 0.01 true))
            (set `self.Timer 0` _returnvalue_2)))))
    (:`then_1`
      (bind _returnvalue_3 (`self.Check component` (`self.Button2`))
        (:`component `
          (if _returnvalue_3
            (bind _returnvalue_4 (`KismetSystemLibrary.K2_SetTimerDelegate` (delegate `RotFunction`) 0.01 true))
            (set `self.Timer 1` _returnvalue_4)))))
    (:`then_2`
      (bind _returnvalue_5 (`self.Check component` (`self.Button3`))
        (:`component `
          (if _returnvalue_5
            (bind _returnvalue_6 (`KismetSystemLibrary.K2_SetTimerDelegate` (delegate `RotFunction2`) 0.01 true))
            (set `self.Timer2` _returnvalue_6)))))
    (:`then_3`
      (bind _returnvalue_7 (`self.Check component` (`self.Button4`))
        (:`component `
          (if _returnvalue_7
            (bind _returnvalue_8 (`KismetSystemLibrary.K2_SetTimerDelegate` (delegate `RotFunction3`) 0.01 true))
            (set `self.Timer3` _returnvalue_8)))))))

(event `RotFunction2`
  (bind _truewheelstates_ (`self.TrueWheelStates `))
  (bind _layer_3 (`self.Layer 3`))
  (bind _finish (`self.RotFunction()` (`self.Timer2`) (`self.Layer3`)))
  (`KismetSystemLibrary.Delay` 0.75)
  (set `self.Rot` (not _finish))
  (bind _result (`/Engine/EditorBlueprintResources/StandardMacros.IncrementInt` _layer_3)
    (:`  `
      (if (== _result (`self.NumberofRots`))
        (set `self.Layer 3` 0)
        (`KismetArrayLibrary.Array_Set` (`self.TrueWheelStates `) 2)
        (elif (== _layer_3 6)
          (`KismetArrayLibrary.Array_Set` _truewheelstates_ 2 true)
          (`self.CheckAll()`)
          (else
            (`KismetArrayLibrary.Array_Set` _truewheelstates_ 2)))))))

(event `RotFunction3`
  (bind _layer_4_ (`self.Layer 4 `))
  (bind _truewheelstates_ (`self.TrueWheelStates `))
  (bind _finish (`self.RotFunction()` (`self.Timer3`) (`self.Layer4`)))
  (`KismetSystemLibrary.Delay` 0.75)
  (set `self.Rot` (not _finish))
  (bind _result (`/Engine/EditorBlueprintResources/StandardMacros.IncrementInt` _layer_4_)
    (:`  `
      (if (== _result (`self.NumberofRots`))
        (set `self.Layer 4 ` 0)
        (`KismetArrayLibrary.Array_Set` (`self.TrueWheelStates `) 3)
        (elif (== _layer_4_ 9)
          (`KismetArrayLibrary.Array_Set` _truewheelstates_ 3 true)
          (`self.CheckAll()`)
          (else
            (`KismetArrayLibrary.Array_Set` _truewheelstates_ 3)))))))

(fn `CheckAll()`
  (for _array_element (`self.TrueWheelStates `)
    (if (== _array_element true)
      (`/Engine/EditorBlueprintResources/StandardMacros.IncrementInt` (`self.overallInt`))
      (else
        (`/Engine/EditorBlueprintResources/StandardMacros.DecrementInt` (`self.overallInt`)))))
  (if (== (`self.overallInt`) 4)
    (`KismetSystemLibrary.PrintString` "Puzzle Complete " true true (struct :`R` 1.0 :`G` 0.831943 :`A` 1.0))
    (message `/Game/Prototype/Tech/PuzzleBlueprints/BPI_PuzzleLogic.Activate` (`self.Object to Activate `) null)
    (else
      (set `self.overallInt` 0))))

(fn `RotFunction()`
  (params (Handle :type "TimerHandle Structure (by ref)") (Target :type "SceneComponent Object Reference"))
  (returns (Finish :type Boolean))
  (bind _output_get (set `self.RotationFloat` (+ (`self.RotationFloat`) 1.0)))
  (if (== _output_get (`self.MaxRot`))
    (`KismetSystemLibrary.K2_ClearAndInvalidateTimerHandle` Handle)
    (`KismetSystemLibrary.PrintString` (`KismetStringLibrary.Conv_DoubleToString` (`self.RotationFloat`)))
    (set `self.RotationFloat` 0.0)
    (else
      (`SceneComponent.K2_AddLocalRotation` Target (`KismetMathLibrary.MakeRotator` 0.0 0.0 1.0) false false)
      (return true))))

(fn `UserConstructionScript`)