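; BP_SequenceHandler runs a button-order puzzle that activates a target object once its buttons are pressed in sequence.
; Its construction script builds the expected string by concatenating 1 through the button count.
; Each press appends its number and is prefix-checked against that string, recoloring the button as correct or incorrect.
; Mistakes reset progress and buttons, restoring materials after a delay, while completion sends ActivateMessage through BPI_PuzzleLogic.
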(event `AddToCompare`
  (params (InputInt :type Integer) (PressedButton :type "Actor Object Reference"))
  (`/Engine/EditorBlueprintResources/StandardMacros.IncrementInt` (`self.NumberofButtonsPressed`)
    (:`  `
      (set `self.StringtoCompare` (`KismetStringLibrary.Concat_StrStr` (`self.StringtoCompare`) (`KismetStringLibrary.Conv_IntToString` InputInt)))
      (`self.CheckCompare` PressedButton))))

(event `CheckCompare`
  (params (`Pressed Button` :type "Actor Object Reference"))
  (bind _returnvalue (`self.GetComponentByClass` `Pressed Button` "/Script/Engine.StaticMeshComponent"))
  (if (`KismetStringLibrary.EqualEqual_StrStr` (`KismetStringLibrary.Left` (`self.CompareString`) (`self.NumberofButtonsPressed`)) (`self.StringtoCompare`))
    (`PrimitiveComponent.SetMaterial` _returnvalue 0 "/Game/Prototype/Tech/SequenceButtons/Materials/M_Correct.M_Correct")
    (if (== (`self.NumberofButtonsPressed`) (`self.Sequence Length`))
      (`self.PuzzleComplete`))
    (else
      (`self.PuzzleFailed`)
      (`PrimitiveComponent.SetMaterial` _returnvalue 0 "/Game/Prototype/Tech/SequenceButtons/Materials/M_Incorrect.M_Incorrect")
      (for _array_element (`self.ButtonArray`)
        (bind _asbp_button_sequence (cast `/Game/Prototype/Tech/SequenceButtons/BP_ButtonSequence` _array_element))
        (`/Game/Prototype/Tech/SequenceButtons/BP_ButtonSequence.Reset` _asbp_button_sequence)))))

(event `PuzzleFailed`
  (`KismetSystemLibrary.PrintString` "Incorrect Button Placed")
  (set `self.NumberofButtonsPressed` 0)
  (set `self.StringtoCompare` "")
  (`KismetSystemLibrary.Delay` 1.0)
  (for _array_element (`self.ButtonArray`)
    (`PrimitiveComponent.SetMaterial` (`self.GetComponentByClass` _array_element "/Script/Engine.StaticMeshComponent") 0 "/Game/Prototype/Tech/PuzzleBlueprints/Textures/M_PedistalMat.M_PedistalMat")))

(event `PuzzleComplete`
  (bind _objecttoactivate (`self.ObjectToActivate`))
  (if (`KismetSystemLibrary.DoesImplementInterface` _objecttoactivate "/Game/Prototype/Tech/PuzzleBlueprints/BPI_PuzzleLogic.BPI_PuzzleLogic_C")
    (message `/Game/Prototype/Tech/PuzzleBlueprints/BPI_PuzzleLogic.Activate` _objecttoactivate)))

(fn `UserConstructionScript`
  (bind _comparestring (`self.CompareString`))
  (set `self.Sequence Length` (`KismetArrayLibrary.Array_Length` (`self.ButtonArray`)))
  (for _index (range 1 (+ (`self.Sequence Length`) 1))
    (set `self.CompareString` (`KismetStringLibrary.Concat_StrStr` _comparestring (`KismetStringLibrary.Conv_IntToString` _index))))
  (`KismetSystemLibrary.PrintString` _comparestring))