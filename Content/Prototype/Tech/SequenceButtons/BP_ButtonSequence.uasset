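; BP_ButtonSequence is a pressable button prototype for a sequence puzzle, coordinated by a BP_SequenceHandler.
; On interaction, an unpressed button latches as pressed, reports its place in the sequence and itself to the handler, and plays a timeline that slides its cube along local X.
; Reset waits briefly, then clears the pressed state and reverses the timeline to pop the button back out.
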(event `/Game/Prototype/Tech/PuzzleBlueprints/BPI_Interaction.InteractWithInteractable`
  (params (HitComponant :type "PrimitiveComponent Object Reference"))
  (if (not (`self.Pressed?`))
    (set `self.Pressed?` true)
    (bind _asbp_sequence_handler (cast `/Game/Prototype/Tech/SequenceButtons/BP_SequenceHandler` (`self.Handler`)))
    (`/Game/Prototype/Tech/SequenceButtons/BP_SequenceHandler.AddToCompare` _asbp_sequence_handler (`self.place in sequence`) self)
    (bind (_direction _newtrack_0) (`Timeline|ButtonPushMovement` :!via `PlayFromStart` :!label _label)
      (:`Update`
        (`SceneComponent.K2_SetRelativeLocation` (`self.Cube`) (`KismetMathLibrary.MakeVector` _newtrack_0) false false)))))

(event `Reset`
  (`KismetSystemLibrary.Delay` 1.2)
  (if (`self.Pressed?`)
    (set `self.Pressed?` false)
    (goto _label :!via `ReverseFromEnd`)))

(fn `UserConstructionScript`)