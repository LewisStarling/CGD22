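; BP_Weight is a weighted prop, apparently for the weight pressure plate prototype.
; Its Weight value picks the mesh in the construction script, from skulls, rock and pottery to weapons, and is exposed through the TheWeight function.
; Construction also applies the asset scale and box extent.
; BeginPlay stores the start location, which this Blueprint never reads, and the box overlap event is empty.
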(event `self.ReceiveBeginPlay`
  (set `self.Start Location` (`self.K2_GetActorLocation`)))

(event `self.Box.OnComponentBeginOverlap`
  (params (OverlappedComponent :type "PrimitiveComponent Object Reference") (OtherActor :type "Actor Object Reference") (OtherComp :type "PrimitiveComponent Object Reference") (OtherBodyIndex :type Integer) (bFromSweep :type Boolean) (SweepResult :type "HitResult Structure (by ref)")))

(fn `TheWeight`
  (returns (OutWeight :type Integer))
  (return (`self.Weight`)))

(fn `UserConstructionScript`
  (bind _cube (`self.Cube`))
  (`StaticMeshComponent.SetStaticMesh` _cube (select `int` (`self.Weight`) :`0` "/Game/Prototype/Art/Art_assets/Mesh/WeightedObject_Skull_Decimated.WeightedObject_Skull_Decimated" :`1` "/Game/Prototype/Art/Art_assets/Mesh/weighted_items/WeightedObject_Skull_Mesh.WeightedObject_Skull_Mesh" :`2` "/Game/Prototype/Art/Art_assets/Mesh/WeightedObejct_Rock.WeightedObejct_Rock" :`3` "/Game/Prototype/Art/Art_assets/Mesh/WeightedObject_Vase.WeightedObject_Vase" :`4` "/Game/Prototype/Art/Art_assets/Mesh/Urn1.Urn1" :`5` "/Game/Prototype/Art/Art_assets/Mesh/Urn2.Urn2" :`6` "/Game/Prototype/Art/Art_assets/Mesh/Axe.Axe" :`7` "/Game/Prototype/Art/Art_assets/Mesh/WallSnakeHead.WallSnakeHead" :`8` "/Game/Prototype/Art/Art_assets/Mesh/Knife_Object.Knife_Object" :!type "StaticMesh Object Reference"))
  (`SceneComponent.SetWorldScale3D` _cube (`self.AssetScale`))
  (`BoxComponent.SetBoxExtent` (`self.Box`) (`self.In Box Extent`) true))