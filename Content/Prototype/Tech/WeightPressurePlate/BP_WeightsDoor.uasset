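; Door for the weight pressure plate puzzle that opens only when the plate holds exactly the required weight.
; On Activate it queries the referenced plate for total and required weight, playing the open timeline on a match if unlocked, or a slight-open timeline on a mismatch.
; Deactivate reverses the open timeline, which moves the hinge along Z with an X rumble, using swept movement.
; Its own weight query functions are stubs returning zero.
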(event `/Game/Prototype/Tech/PuzzleBlueprints/BPI_PuzzleLogic.Deactivate`
  ;[1 1 1] Door opens
  (bind (_direction _dooraxis _doorrumble) (`Timeline|DoorOpen` :!via `Reverse` :!label _label)
    (:`Update`
      (`SceneComponent.K2_SetRelativeLocation` (`self.Hinge`) (`KismetMathLibrary.MakeVector` _doorrumble 0.0 _dooraxis) true false))))

(event `/Game/Prototype/Tech/PuzzleBlueprints/BPI_PuzzleLogic.Activate`
  (params (`component ` :type "SceneComponent Object Reference"))
  ;[1 1 1] Door opens
  (bind (_reqweight _totweight) (message `/Game/Prototype/Tech/WeightPressurePlate/BPI_Weights.weightforDoor` (`self.PressurePlateRef`)))
  (if (== _totweight _reqweight)
    (if (not (`self.Locked?`))
      (goto _label))
    (else
      (bind (_direction _doorslightopen) (`Timeline|DoorSlightOpen` :!via `PlayFromStart`)
        (:`Update`
          (`SceneComponent.K2_SetRelativeLocation` (`self.Hinge`) (`KismetMathLibrary.MakeVector` 0.0 0.0 _doorslightopen) true false))))))

(fn `TheWeight`
  (returns (OutWeight :type Integer))
  (return 0))

(fn `UserConstructionScript`)

(fn `weightforDoor`
  (returns (ReqWeight :type Integer) (TotWeight :type Integer))
  (return 0 0))