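; BP_RiddleNote is an interactable note actor that shows a riddle to the player.
; Its construction script writes the note's Text onto a TextRender component, and BeginPlay caches the level's BP_UIManager.
; When an interaction hits the Plane component, it adds the manager's RiddleNote widget to the viewport with that text, then removes it after a fixed delay.
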(event `self.ReceiveBeginPlay`
  (bind _returnvalue (`GameplayStatics.GetActorOfClass` "/Game/Prototype/Tech/UI-UX/BP_UIManager.BP_UIManager_C"))
  (set `self.UI Manager` _returnvalue))

(event `/Game/Prototype/Tech/PuzzleBlueprints/BPI_Interaction.InteractWithInteractable`
  (params (HitComponant :type "PrimitiveComponent Object Reference"))
  (bind _riddle_note_ (`/Game/Prototype/Tech/UI-UX/BP_UIManager.Riddle note ` (`self.UI Manager`)))
  (if (== HitComponant (`self.Plane`))
    (`UserWidget.AddToViewport` _riddle_note_ 0)
    (`TextBlock.SetText` (`/Game/Prototype/Tech/UI-UX/W_RiddleNote.T_RiddleText` _riddle_note_) (`self.Text`))
    (`KismetSystemLibrary.Delay` 4.0)
    (`Widget.RemoveFromParent` _riddle_note_)))

(fn `UserConstructionScript`
  (`TextRenderComponent.K2_SetText` (`self.TextRender`) (`self.Text`)))